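; Player controller for a team-based game that handles team selection and player spawning.
; On BeginPlay, the local controller shows the W_TeamSelection widget.
; Its SpawnPlayer event takes a team tag and hands it, with the controller, to TeamGameMode for spawning.
; For Team2 only, that event then adds the W_Objectives widget to the player screen.
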(event Custom|SpawnPlayer
  (params (TeamTag :type Name))
  (bind _asteam_game_mode (Utilities|Casting|CastToTeamGameMode (Game|GetGameMode)))
  (Default|SpawnPlayer _asteam_game_mode TeamTag self)
  (if (== TeamTag "Team2")
    (bind _returnvalue (UserInterface|CreateWidget "/Game/Widgets/W_Objectives.W_Objectives_C"))
    (UserInterface|Viewport|AddtoPlayerScreen _returnvalue)))

(event EventBeginPlay
  (if (Pawn|IsLocalPlayerController)
    (bind _returnvalue (UserInterface|CreateWidget "/Game/Widgets/W_TeamSelection.W_TeamSelection_C"))
    (UserInterface|Viewport|AddtoViewport _returnvalue 0)))

(fn ConstructionScript)